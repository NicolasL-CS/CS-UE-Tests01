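; AI patrol path point actor that marks a spot for patrolling pawns and signals when one reaches it.
; On patroller entry, it fires the OnPointReached dispatcher, then sets the pawn controller's control rotation to the point arrow's world rotation, so the arrow defines the facing at that point.
; The construction script applies the HiddenInGame flag to the marker mesh and arrow.
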(event Custom|OnPatrollerEntered
  (params (Pawn :type Pawn%20Object%20Reference))
  (Variables|Default|SetPawn_Controller (Pawn|GetController Pawn))
  (Default|CallOnPointReached)
  (Utilities|FlowControl|Sequence
    (:then_0
      (Pawn|SetControlRotation (Variables|Default|GetPawn_Controller) (Transformation|GetWorldRotation (Variables|Default|GetPoint_Arrow))))))

(fn ConstructionScript
  (Development|SetHiddeninGame (Variables|Default|GetPoint_Mesh) (Variables|Default|GetHiddenInGame?) false)
  (Development|SetHiddeninGame (Variables|Default|GetPoint_Arrow) (Variables|Default|GetHiddenInGame?) false))